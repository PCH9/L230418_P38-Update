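; BP_P39_Pawn is a player-controlled plane pawn that flies forward continuously.
; Tick adds movement input along the actor's forward vector, then spins the left and right propellers through two helper functions.
; Pitch and roll axis inputs apply clamped, delta-time-scaled local rotation to steer the plane.
; An older local-offset method of forward movement remains in the graph but never runs.
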(event EventTick
  (params (DeltaSeconds :type Float%20%28single-precision%29))
  (Utilities|FlowControl|Sequence
    (:then_0
      (Pawn|Input|AddMovementInput (Transformation|GetActorForwardVector) 1.0 false))
    (:then_1
      ;[1 1 1] 왼쪽 프로펠러
      (CallFunction|LeftPropeller (Variables|Default|GetLeft)))
    (:then_2
      ;[1 1 1] 오른쪽 프로펠러
      (CallFunction|RightPropeller (Variables|Default|GetRight)))))

(event Input|AxisEvents|InputAxisPicth
  (params (AxisValue :type Float%20%28single-precision%29))
  (Transformation|AddActorLocalRotation (Math|Rotator|MakeRotator 0.0 (* (Math|Float|Clamp(Float) AxisValue -1.0) (Utilities|Time|GetWorldDeltaSeconds) (Variables|속력|GetPlayerRotateSpeed)) 0.0) false false))

(event Input|AxisEvents|InputAxisRoll
  (params (AxisValue :type Float%20%28single-precision%29))
  (Transformation|AddActorLocalRotation (Math|Rotator|MakeRotator (* (Math|Float|Clamp(Float) AxisValue -1.0) (Utilities|Time|GetWorldDeltaSeconds) (Variables|속력|GetPlayerRotateSpeed)) 0.0 0.0) false false))

(fn ConstructionScript)

(fn LeftPropeller
  (params (self2 :type Scene%20Component%20Object%20Reference))
  (Transformation|AddRelativeRotation self2 (Math|Rotator|MakeRotator (* (Utilities|Time|GetWorldDeltaSeconds) (Variables|속력|GetPropeller%20Rotate%20Speed)) 0.0 0.0) false false))

(fn RightPropeller
  (params (self2 :type Scene%20Component%20Object%20Reference))
  (Transformation|AddRelativeRotation self2 (Math|Rotator|MakeRotator (* (Utilities|Time|GetWorldDeltaSeconds) (Variables|속력|GetPropeller%20Rotate%20Speed)) 0.0 0.0) false false))