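; BP_P38 is a P-38 aircraft actor that flies forward on its own while spinning its two propellers.
; Each Tick moves the actor along its local X axis at P38Speed, scaled by delta time.
; Two helper functions, one per side, add frame-rate-independent roll rotation to the Left and Right propeller components using a shared PropellerRotateSpeed.
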(event EventTick
  (params (DeltaSeconds :type Float%20%28single-precision%29))
  (Utilities|FlowControl|Sequence
    (:then_0
      ;[1 1 1] X축으로 전진
      (Transformation|AddActorLocalOffset (Math|Vector|MakeVector (* (Utilities|Time|GetWorldDeltaSeconds) (Variables|속력|GetP38%20Speed)) 0.0 0.0) false false))
    (:then_1
      ;[1 1 1] 왼쪽 프로펠러
      (CallFunction|LeftPropeller (Variables|Default|GetLeft)))
    (:then_2
      ;[1 1 1] 오른쪽 프로펠러
      (CallFunction|RightPropeller (Variables|Default|GetRight)))))

(fn ConstructionScript)

(fn LeftPropeller
  (params (self2 :type Scene%20Component%20Object%20Reference))
  (Transformation|AddRelativeRotation self2 (Math|Rotator|MakeRotator (* (Utilities|Time|GetWorldDeltaSeconds) (Variables|속력|GetPropeller%20Rotate%20Speed)) 0.0 0.0) false false))

(fn RightPropeller
  (params (self2 :type Scene%20Component%20Object%20Reference))
  (Transformation|AddRelativeRotation self2 (Math|Rotator|MakeRotator (* (Utilities|Time|GetWorldDeltaSeconds) (Variables|속력|GetPropeller%20Rotate%20Speed)) 0.0 0.0) false false))